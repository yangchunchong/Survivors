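; Player controller for the main menu lobby that sets the game language and shows the main menu UI.
; On BeginPlay it applies the language from the PlayerSetting save, or the current culture if no save exists.
; For the local controller it then creates the WB_MainMenu widget, adds it to the viewport and switches to UI-only input.
; UpdateCharacterInfo pushes experience progress and level text into the menu's talent screen.
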(event EventBeginPlay
  ;[0.1094 0.1094 0.1094] Prepare Lobby UI
  (CallFunction|SetLanguage)
  (if (Pawn|IsLocalPlayerController)
    (Variables|Default|GetMainMenu
      (:then
        _)
      (:else
        (bind _returnvalue (UserInterface|CreateWidget "/Game/SurvivorsTemplate/Widgets/WB_MainMenu.WB_MainMenu_C" self))
        (Variables|Default|SetMainMenu _returnvalue)))
    (UserInterface|Viewport|AddtoViewport (Variables|Default|GetMainMenu) 0)
    (Input|SetInputModeUIOnly self 0 "DoNotLock" false)))

(fn ConstructionScript)

(fn UpdateCharacterInfo
  (params (InPercent :type Float%20%28single-precision%29) (InText :type Text))
  (bind _mainmenu (Variables|Default|GetMainMenu))
  (bind _talentmenu (Variables|/Game/SurvivorsTemplate/Widgets/WB_MainMenu.WB_MainMenu_C|GetTalentMenu _mainmenu))
  (Progress|SetPercent (Variables|/Game/SurvivorsTemplate/Widgets/WB_TalentMenu.WB_TalentMenu_C|GetCharacterExp _talentmenu) InPercent)
  (Rendering|Components|TextRender|SetText (Variables|/Game/SurvivorsTemplate/Widgets/WB_TalentMenu.WB_TalentMenu_C|GetCharacterLevelLabel _talentmenu) InText))

(fn SetLanguage
  (bind _returnvalue (Utilities|Internationalization|GetCurrentCulture))
  (bind _returnvalue_2 (SaveGame|DoesSaveGameExist "PlayerSetting"))
  (if _returnvalue_2
    (bind _returnvalue_3 (SaveGame|LoadGamefromSlot "PlayerSetting"))
    (bind _asbp_sg_setting (Utilities|Casting|CastToBP_SG_Setting _returnvalue_3))
    (Class|KismetInternationalizationLibrary|SetCurrentLanguage (Variables|/Game/SurvivorsTemplate/Blueprints/Saves/BP_SG_Setting.BP_SG_Setting_C|GetSystemLanguage _asbp_sg_setting))
    (else
      (Development|PrintString (Utilities|String|Append _returnvalue "   ---------   "))
      (Class|KismetInternationalizationLibrary|SetCurrentLanguage _returnvalue)
      (Development|PrintString (Utilities|String|Append (Class|KismetInternationalizationLibrary|GetCurrentLanguage) "   ---------   ")))))