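; Player character Blueprint for the Survivors template game, adding debug inputs for hiding the HUD and the character.
; The GodMode input toggles an IsGodMode flag, which gates the other two actions.
; ShowHUD switches the gameplay player controller's HUD between hidden and visible, while ShowCharacter toggles the mesh and its children.
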(event EventBeginPlay
  (|CallParentFunction) ; This node is disabled and will not be called.\nDrag off pins to build functionality.
)

(event Collision|EventActorBeginOverlap
  (params (OtherActor :type Actor%20Object%20Reference)))

(event EventTick
  (params (DeltaSeconds :type Float%20%28single-precision%29)))

(event Input|ActionEvents|InputActionShowHUD
  (params (Key :type Key%20Structure :default "None"))
  ;[1 1 1] ShowHUD
  (:Pressed
    (if (Variables|Debug|GetbIsGodMode)
      (bind _asbp_gameplay_player_controller (Utilities|Casting|CastToBP_Gameplay_PlayerController (Pawn|GetController)))
      (switch Utilities|FlowControl|Switch|SwitchonESlateVisibility (Widget|GetVisibility (Variables|/Game/SurvivorsTemplate/Blueprints/System/BP_Gameplay_PlayerController.BP_Gameplay_PlayerController_C|GetPlayerHud _asbp_gameplay_player_controller))
        (:Visible
          (Widget|SetVisibility (Variables|/Game/SurvivorsTemplate/Blueprints/System/BP_Gameplay_PlayerController.BP_Gameplay_PlayerController_C|GetPlayerHud _asbp_gameplay_player_controller) "Hidden" :!label _label))
        (:Hidden
          (Widget|SetVisibility (Variables|/Game/SurvivorsTemplate/Blueprints/System/BP_Gameplay_PlayerController.BP_Gameplay_PlayerController_C|GetPlayerHud _asbp_gameplay_player_controller) "SelfHitTestInvisible"))
        (:HitTestInvisible
          (goto _label))
        (:SelfHitTestInvisible
          (goto _label))))))

(event Input|ActionEvents|InputActionShowCharacter
  (params (Key :type Key%20Structure :default "None"))
  (bind _mesh (Variables|Character|GetMesh))
  ;[1 1 1] ShowCharacter
  (:Pressed
    (if (Variables|Debug|GetbIsGodMode)
      (Rendering|SetVisibility _mesh (not (Variables|/Script/Engine.SceneComponent|GetbVisible _mesh)) true))))

(event Input|ActionEvents|InputActionGodMode
  (params (Key :type Key%20Structure :default "None"))
  ;[1 1 1] GodMode
  (:Pressed
    (Variables|Debug|SetbIsGodMode (not (Variables|Debug|GetbIsGodMode)))))

(fn ConstructionScript
  (|CallParentFunction))