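; Modular samurai sample character from an Asian armour pack, built from skeletal mesh body and gear parts plus static meshes for each hand.
; The construction script makes the parts follow the inherited Mesh as leader pose and attaches the hand meshes to its sockets.
; Boolean equipment and face options become 0/1 morph targets applied across all parts, reapplied on BeginPlay because "Use Animation Asset" mode prevents setting them at construction.
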(event EventBeginPlay
  ;[1 1 1] Update Morph Targets again, since we can not set them in Construction Script with Animation Mode "Use Animation Asset"
  (CallFunction|UpdateMorphTargets))

(fn ConstructionScript
  (Variables|Customization|SetRefresh false)
  (CallFunction|UpdateMorphTargets)
  (CallFunction|SetMasterPoseComponentforParts))

(fn SetMasterPoseComponentforParts
  (bind _sk_armour_extra (Variables|Components|GetSK_Armour_Extra))
  ;[0 0 0] Updates all Part components (skeletal and static meshes) to follow the Master Pose of Mesh (Inherited).
  ;
  ; This means, you can set the character's animation in its editor Details Panel or in Mesh (Inherited) component itself, which then gets used for all other Part components as well automatically.
  (Utilities|FlowControl|Sequence
    (:then_0
      (Components|SkinnedMesh|SetLeaderPoseComponent _sk_armour_extra (Variables|Character|GetMesh) false false)
      (Transformation|AttachComponentToComponent (Variables|Components|GetSM_LeftHand) (Variables|Character|GetMesh) "LeftHandSocket" "KeepRelative" "KeepRelative" "KeepRelative" true)
      (Transformation|AttachComponentToComponent (Variables|Components|GetSM_RightHand) (Variables|Character|GetMesh) "RightHandSocket" "KeepRelative" "KeepRelative" "KeepRelative" true))
    (:then_1
      (for _array_element (Utilities|Array|MakeArray (Variables|Components|GetSK_Hair) (Variables|Components|GetSK_Head) (Variables|Components|GetSK_Chest) (Variables|Components|GetSK_Hand/Glove) _sk_armour_extra (Variables|Components|GetSK_Pants) (Variables|Components|GetSK_Boots) (Variables|Components|GetSK_Skin_Extra) (Variables|Components|GetSK_Hat))
        (if (Utilities|IsValid (Variables|/Script/Engine.SkeletalMeshComponent|GetSkeletalMeshAsset _array_element))
          (if (not (or (Utilities|IsValidClass (Variables|/Script/Engine.SkeletalMeshComponent|GetAnimClass _array_element)) (Utilities|IsValidClass (Variables|/Script/Engine.SkeletalMesh|GetPostProcessAnimBlueprint (Variables|/Script/Engine.SkeletalMeshComponent|GetSkeletalMeshAsset _array_element)))))
            (Components|SkinnedMesh|SetLeaderPoseComponent _array_element (Variables|Character|GetMesh) false false)))))))

(fn GetMorphTargetValue
  (params (CanMorph :type Boolean))
  (return (Math|Float|SelectFloat 1.0 0.0 CanMorph)))

(fn UpdateMorphTargets
  (bind _sk_boots (Variables|Components|GetSK_Boots))
  (bind _sk_skin_extra (Variables|Components|GetSK_Skin_Extra))
  (bind _sk_pants (Variables|Components|GetSK_Pants))
  (bind _sk_hair (Variables|Components|GetSK_Hair))
  (bind _sk_hat (Variables|Components|GetSK_Hat))
  (bind _sk_head (Variables|Components|GetSK_Head))
  (bind _sk_hand_glove (Variables|Components|GetSK_Hand/Glove))
  (bind _sk_armour_extra (Variables|Components|GetSK_Armour_Extra))
  (bind _sk_chest (Variables|Components|GetSK_Chest))
  (bind _array (Utilities|Array|MakeArray _sk_hat _sk_hair _sk_head _sk_chest _sk_hand_glove _sk_armour_extra _sk_skin_extra _sk_boots _sk_pants))
  (for _array_element _array
    (Utilities|IsValid _array_element
      (:Is%20Valid
        (Components|SkeletalMesh|SetMorphTarget _array "hat_equipped" (CallFunction|GetMorphTargetValue (Variables|Customization|MorphTargets|GetHatEquipped)) true)
        (Components|SkeletalMesh|SetMorphTarget _array "gloves_equipped" (CallFunction|GetMorphTargetValue (Variables|Customization|MorphTargets|GetGlovesEquipped)) true)
        (Components|SkeletalMesh|SetMorphTarget _array_element "hat_equipped" (CallFunction|GetMorphTargetValue (Variables|Customization|MorphTargets|GetHatEquipped)) true)
        (Components|SkeletalMesh|SetMorphTarget _array_element "gloves_equipped" (CallFunction|GetMorphTargetValue (Variables|Customization|MorphTargets|GetGlovesEquipped)) true)
        (Components|SkeletalMesh|SetMorphTarget _array_element "pants_long_equipped" (CallFunction|GetMorphTargetValue (Variables|Customization|MorphTargets|Getpants_equipped)) true)
        (Components|SkeletalMesh|SetMorphTarget _array_element "Collar_high" (CallFunction|GetMorphTargetValue (Variables|Customization|MorphTargets|Getcollar_high)) true)
        (Components|SkeletalMesh|SetMorphTarget _array_element "skirt_long_equipped" (CallFunction|GetMorphTargetValue (Variables|Customization|MorphTargets|GetRobe_equipped)) true)
        (Components|SkeletalMesh|SetMorphTarget _array_element "pants_equipped" (CallFunction|GetMorphTargetValue (Variables|Customization|MorphTargets|Getpants_equipped)) true)
        (Components|SkeletalMesh|SetMorphTarget _array_element "boot_high_equipped" (CallFunction|GetMorphTargetValue (Variables|Customization|MorphTargets|Getboot_high_equipped)) true)
        (Components|SkeletalMesh|SetMorphTarget _array_element "face_02" (CallFunction|GetMorphTargetValue (Variables|Customization|Head|Getface_02)) true)
        (Components|SkeletalMesh|SetMorphTarget _array "face_03" (CallFunction|GetMorphTargetValue (Variables|Customization|Head|Getface_03)) true)
        (Components|SkeletalMesh|SetMorphTarget _array "face_04" (CallFunction|GetMorphTargetValue (Variables|Customization|Head|Getface_04)) true)))))